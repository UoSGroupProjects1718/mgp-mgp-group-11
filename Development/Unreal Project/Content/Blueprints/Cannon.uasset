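; Turn-based two-player cannon that swings back and forth between pitch limits and fires a Bullet on touch or Fire input.
; Tick pauses while a bullet exists or the game is over; otherwise it aims a laser beam by line trace and sweeps the cannon.
; Firing flags a turn change, which a FlipFlop applies once the bullet is gone, updating BounceGamemode, score circles and cannon material.
; An unfinished turn timer is left unconnected.
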(event EventTick
  (params (DeltaSeconds :type Float%20%28single-precision%29))
  (bind _returnvalue (Game|GetGameMode))
  (bind _returnvalue_2 (Game|GetGameMode))
  (bind _returnvalue_3 (Transformation|GetActorRotation))
  (bind _papersprite (Variables|Default|GetPaperSprite))
  (bind _arrow (Variables|Default|GetArrow))
  (bind _returnvalue_4 (Transformation|GetWorldLocation _arrow))
  (bind _asbounce_gamemode (Utilities|Casting|CastToBounceGamemode _returnvalue))
  (bind _asbounce_gamemode_2 (Utilities|Casting|CastToBounceGamemode _returnvalue_2))
  (bind _widgetvar (Variables|/Game/Blueprints/BounceGamemode.BounceGamemode_C|GetWidgetVar _asbounce_gamemode_2))
  (bind _scorecircle1 (Variables|/Game/Blueprints/Widgets/HUDWidget.HUDWidget_C|GetScoreCircle1 _widgetvar))
  (bind _scorecircle2 (Variables|/Game/Blueprints/Widgets/HUDWidget.HUDWidget_C|GetScoreCircle2 _widgetvar))
  (Variables|Default|SetDeltaSeconds DeltaSeconds)
  ;[1 1 1] Pause while firing
  (bind _outactors (Actor|GetAllActorsOfClass "/Game/Blueprints/Bullet.Bullet_C"))
  (if (and (<= (Utilities|Array|Length _outactors) 0) (not (Variables|/Game/Blueprints/BounceGamemode.BounceGamemode_C|GetGameIsOver (.AsBounce%20Gamemode (Utilities|Casting|CastToBounceGamemode (Game|GetGameMode))))))
    ;[1 1 1] Show Laser Pointer
    (Rendering|SetVisibility (Variables|Default|GetParticleSystem) true false)
    ;[1 1 1] Draw Raytrace
    (bind _outactors_2 (Actor|GetAllActorsOfClass "/Game/Blueprints/Bullet.Bullet_C"))
    (bind _outhit (Collision|LineTraceByChannel _returnvalue_4 (+ _returnvalue_4 (* (Math|Vector|GetForwardVector (Transformation|GetWorldRotation _arrow)) 2e+03)) "TraceTypeQuery1" false _outactors_2 "None"))
    (Class|ParticleSystemComponent|SetBeamTargetPoint (Variables|Default|GetParticleSystem) 0 (.location _outhit))
    ;[1 1 1] Set Which Players turn it is
    (if (Variables|Default|GetCheckToChangeTurn)
      (Utilities|FlowControl|FlipFlop
        (:A
          (Variables|/Game/Blueprints/BounceGamemode.BounceGamemode_C|SetPlayer1Turn _asbounce_gamemode false)
          (Appearance|SetBrushfromTexture _scorecircle1 "/Game/Textures/HUDPictures/ScoreCircleDisabled.ScoreCircleDisabled" false)
          (Appearance|SetBrushfromTexture _scorecircle2 "/Game/Textures/HUDPictures/ScoreCircleRed.ScoreCircleRed" false)
          (Rendering|Material|SetMaterial _papersprite 0 "/Game/Materials/Player2Cannon.Player2Cannon"))
        (:B
          (Variables|/Game/Blueprints/BounceGamemode.BounceGamemode_C|SetPlayer1Turn _asbounce_gamemode true)
          (Appearance|SetBrushfromTexture _scorecircle1 "/Game/Textures/HUDPictures/ScoreCircleBlue.ScoreCircleBlue" false)
          (Appearance|SetBrushfromTexture _scorecircle2 "/Game/Textures/HUDPictures/ScoreCircleDisabled.ScoreCircleDisabled" false)
          (Rendering|Material|SetMaterial _papersprite 0 "/Game/Materials/Player1Cannon.Player1Cannon")))
      (Variables|Default|SetCheckToChangeTurn false))
    ;[1 1 1] Cannon Movement
    ;;[1 1 1] Restrain Cannon between 60 and -60
    (if (>= (.pitch _returnvalue_3) 6e+01)
      (Variables|Default|SetDirection -1.0)
      (elif (<= (.pitch _returnvalue_3) -6e+01)
        (Variables|Default|SetDirection 1.0)))
    (Transformation|SetActorRotation (Math|Rotator|MakeRotator 0.0 (+ (* (Variables|Default|GetDeltaSeconds) (Variables|Default|GetSpeed) (Variables|Default|GetDirection)) (.pitch _returnvalue_3)) 0.0))))

(event Input|ActionEvents|InputActionFire
  (params (Key :type Key%20Structure))
  (:Pressed
    ;[1 1 1] Cant fire if bullet is active
    (bind _outactors (Actor|GetAllActorsOfClass "/Game/Blueprints/Bullet.Bullet_C"))
    (if (and (<= (Utilities|Array|Length _outactors) 0) (not (Variables|/Game/Blueprints/BounceGamemode.BounceGamemode_C|GetGameIsOver (.AsBounce%20Gamemode (Utilities|Casting|CastToBounceGamemode (Game|GetGameMode))))))
      ;[1 1 1] Disable Laser Pointer
      (Rendering|SetVisibility (Variables|Default|GetParticleSystem) false false)
      ;[1 1 1] Spawn Bullet
      (Audio|PlaySound2D 0)
      (bind _returnvalue (Game|SpawnActorfromClass "/Game/Blueprints/Bullet.Bullet_C" (Transformation|GetWorldTransform (Variables|Default|GetArrow)) "AlwaysSpawn" 0 0))
      (Variables|Default|SetCheckToChangeTurn true)
      (Variables|Default|SetBulletRef _returnvalue))))

(event Input|TouchEvents|InputTouch
  (params (Location :type Vector) (FingerIndex :type ETouchIndex%20Enum))
  (:Pressed
    ;[1 1 1] Cant fire if bullet is active
    (bind _outactors (Actor|GetAllActorsOfClass "/Game/Blueprints/Bullet.Bullet_C"))
    (if (and (<= (Utilities|Array|Length _outactors) 0) (not (Variables|/Game/Blueprints/BounceGamemode.BounceGamemode_C|GetGameIsOver (.AsBounce%20Gamemode (Utilities|Casting|CastToBounceGamemode (Game|GetGameMode))))))
      ;[1 1 1] Disable Laser Pointer
      (Rendering|SetVisibility (Variables|Default|GetParticleSystem) false false)
      ;[1 1 1] Spawn Bullet
      (Audio|PlaySound2D 0)
      (bind _returnvalue (Game|SpawnActorfromClass "/Game/Blueprints/Bullet.Bullet_C" (Transformation|GetWorldTransform (Variables|Default|GetArrow)) "AlwaysSpawn" 0 0))
      (Variables|Default|SetCheckToChangeTurn true)
      (Variables|Default|SetBulletRef _returnvalue))))

(fn ConstructionScript)