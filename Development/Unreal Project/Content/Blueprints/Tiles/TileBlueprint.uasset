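; A Paper2D tile actor with three types, normal, blocker and breakable, that reacts to bullet hits and can patrol waypoints.
; The construction script picks the sprite material from the tile type.
; Tick moves it at constant speed with sweep between waypoints, reversing at either end.
; Bullet hits spawn particles in the tile's material; blockers destroy the bullet, while breakables destroy themselves after a brief delay.
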(event OnComponentHit(PaperSprite)
  (params (HitComponent :type Primitive%20Component%20Object%20Reference) (OtherActor :type Actor%20Object%20Reference) (OtherComp :type Primitive%20Component%20Object%20Reference) (NormalImpulse :type Vector :default "0, 0, 0") (Hit :type Hit%20Result%20Structure%20%28by%20ref%29))
  (bind _tiletype (Variables|Default|GetTileType))
  (if (== (Utilities|GetClass OtherActor) "/Game/Blueprints/Bullet.Bullet_C")
    (bind _returnvalue (Effects|SpawnEmitteratLocation "/Game/Particles/CollisionParticles.CollisionParticles" (.location Hit) (Math|Conversions|RotationFromXVector (* (.normal Hit) -1))))
    (Rendering|Material|SetMaterial _returnvalue 0 (Rendering|Material|GetMaterial HitComponent 0))
    ;[1 1 1] NormalTile
    (if (not (== _tiletype 0))
      ;[1 1 1] BlockerTile
      (if (== _tiletype 1)
        (Actor|DestroyActor OtherActor)
        (else
          ;[1 1 1] Breakable Tile
          (if (== _tiletype 2)
            (Utilities|FlowControl|Delay 0.05)
            (Actor|DestroyActor)))))))

(event EventTick
  (params (DeltaSeconds :type Float%20%28single-precision%29))
  (bind _returnvalue (Transformation|GetActorLocation))
  ;[1 1 1] Lerp target between waypoints
  (if (!= (Utilities|Array|Length (Variables|Default|GetWaypoints)) 0)
    (if (Math|Vector|Equal(Vector) _returnvalue (Transformation|GetActorLocation (Utilities|Array|Get(acopy) (Variables|Default|GetWaypoints) (Variables|Default|GetCurrentWaypoint))) 0.1)
      ;[1 1 1] Cycle waypoint
      (Variables|Default|SetCurrentWaypoint (+ (Variables|Default|GetCurrentWaypoint) (Variables|Default|GetWaypointDirection)))
      ;[1 1 1] If at end of waypoints, go the other way
      (if (or (== (Variables|Default|GetCurrentWaypoint) 0) (== (Variables|Default|GetCurrentWaypoint) (- (Utilities|Array|Length (Variables|Default|GetWaypoints)) 1)))
        (Variables|Default|SetWaypointDirection (* (Variables|Default|GetWaypointDirection) -1))))
    (Transformation|SetActorLocation (Math|Interpolation|VInterptoConstant _returnvalue (Transformation|GetActorLocation (Utilities|Array|Get(acopy) (Variables|Default|GetWaypoints) (Variables|Default|GetCurrentWaypoint))) DeltaSeconds (Variables|Default|GetSpeed)) true false)))

(fn ConstructionScript
  (Rendering|Material|SetMaterial (Variables|Default|GetPaperSprite) 0 (Utilities|Select :Index (Variables|Default|GetTileType) :Option%200 "/Game/Materials/NormalTileMaterial.NormalTileMaterial" :Option%201 "/Game/Materials/BlockerTileMaterial.BlockerTileMaterial" :Option%202 "/Game/Materials/BreakableTileMaterial.BreakableTileMaterial")))