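; Player-controlled turret for a two-player, turn-based shooter that automatically sweeps its pitch up and down between fixed limits.
; Tick steps the rotation using a DoOnce reset after a short Delay, with a boolean flipping direction at each limit.
; Space spawns a Bullet from the Arrow component, swaps the turn shown on the HUD created at BeginPlay, and blocks firing during a brief cooldown.
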(event EventTick
  (params (DeltaSeconds :type Float%20%28single-precision%29))
  (bind _returnvalue (Transformation|GetActorTransform))
  (bind _returnvalue_2 (Transformation|GetActorTransform))
  (bind (_location _rotation _scale) (Math|Transform|BreakTransform _returnvalue))
  (bind (_location_2 _rotation_2 _scale_2) (Math|Transform|BreakTransform _returnvalue_2))
  (bind (_roll _pitch _yaw) (Math|Rotator|BreakRotator _rotation))
  (bind (_roll_2 _pitch_2 _yaw_2) (Math|Rotator|BreakRotator _rotation_2))
  (Variables|Default|SetDeltaTime DeltaSeconds)
  (Utilities|FlowControl|DoOnce false :!label _label
    (:Completed
      (if (Variables|Default|GetRotation)
        (if (< _pitch 49.0)
          _
          (else
            (Variables|Default|SetRotation false)
            (Utilities|FlowControl|Delay 0.02 :!label _label_2)
            (Transformation|SetActorTransform (Math|Transform|MakeTransform _location_2 (Math|Rotator|MakeRotator _roll_2 (- _pitch_2 2.0) _yaw_2) _scale_2))
            (goto _label Reset)))
        (elif (> _pitch -5e+01)
          (goto _label_2)
          (else
            (Variables|Default|SetRotation true))))
      (Utilities|FlowControl|Delay 0.02)
      (Transformation|SetActorTransform (Math|Transform|MakeTransform _location (Math|Rotator|MakeRotator _roll (+ _pitch 2.0) _yaw) _scale))
      (goto _label Reset))))

(event EventBeginPlay
  (Input|EnableInput (Game|GetPlayerController 0))
  (bind _returnvalue (UserInterface|CreateWidget "/Game/Blueprints/HUD.HUD_C"))
  (bind _output_get (Variables|Default|SetPlayer%20Turn%20HUD _returnvalue))
  (UserInterface|Viewport|AddtoViewport _output_get 0)
  (Rendering|Components|TextRender|SetText (Variables|/Game/Blueprints/HUD.HUD_C|GetPlayerTurnText _output_get) "Player 1"))

(event Input|KeyboardEvents|SpaceBar
  (params (Key :type Key%20Structure))
  (bind _arrow (Variables|Default|GetArrow))
  (bind _returnvalue (Transformation|GetWorldTransform _arrow))
  (bind (_location _rotation) (Math|Transform|BreakTransform _returnvalue))
  (bind (_roll _pitch _yaw) (Math|Rotator|BreakRotator _rotation))
  (:Pressed
    (if (not (Variables|Default|GetisFiring))
      (Game|SpawnActorfromClass "/Game/Blueprints/Bullet.Bullet_C" (Math|Transform|MakeTransform _location (Math|Rotator|MakeRotator _roll (+ _pitch 9e+01) _yaw)) "Undefined" 0 0)
      (Variables|Default|SetisFiring true)
      (if (Variables|Default|GetPlayer1Turn)
        (Variables|Default|SetPlayer1Turn false)
        (Rendering|Components|TextRender|SetText (Variables|/Game/Blueprints/HUD.HUD_C|GetPlayerTurnText (stale EventBeginPlay _output_get)) "Player 2")
        (else
          (Variables|Default|SetPlayer1Turn true)
          (Rendering|Components|TextRender|SetText (Variables|/Game/Blueprints/HUD.HUD_C|GetPlayerTurnText (stale EventBeginPlay _output_get)) "Player 1")))
      (Utilities|FlowControl|Delay 2.0)
      (Variables|Default|SetisFiring false))))

(fn ConstructionScript)