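; Bullet projectile for a two-player, turn-based bouncing game, limited to a maximum number of bounces.
; Its construction script reads the current turn from BounceGamemode and gives the sphere that player's bullet material.
; Each ProjectileMovement bounce increments a counter and plays a bounce sound, until the limit is reached and the bullet plays a destroy sound and destroys itself.
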(event OnProjectileBounce(ProjectileMovement)
  (params (ImpactResult :type Hit%20Result%20Structure%20%28by%20ref%29) (ImpactVelocity :type Vector%20%28by%20ref%29 :default "0, 0, 0"))
  (bind _output_get (Variables|Default|SetBounces (+ (Variables|Default|GetBounces) 1)))
  (if (>= _output_get (Variables|Default|GetMaxBounces))
    (Audio|PlaySound2D "/Game/Audio/BulletDestroy.BulletDestroy" 1.0 1.0)
    (Actor|DestroyActor)
    (else
      (Audio|PlaySound2D "/Game/Audio/Bounce.Bounce"))))

(fn ConstructionScript
  (bind _sphere (Variables|Default|GetSphere))
  (if (Variables|/Game/Blueprints/BounceGamemode.BounceGamemode_C|GetPlayer1Turn (.AsBounce%20Gamemode (Utilities|Casting|CastToBounceGamemode (Game|GetGameMode))))
    (Rendering|Material|SetMaterial _sphere 0 "/Game/Materials/Player1BulletMaterial.Player1BulletMaterial")
    (else
      (Rendering|Material|SetMaterial _sphere 0 "/Game/Materials/Player2BulletMaterial.Player2BulletMaterial"))))