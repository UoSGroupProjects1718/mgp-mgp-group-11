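; Scoring target for a two-player, turn-based bounce shooter that can patrol between waypoints.
; A sprite hit destroys the other actor and the target, plays particles and a settings-gated sound, and adds a point for the current player in BounceGamemode and its HUD.
; Reaching WinScore flags game over and swaps in a winner screen with both scores.
; Tick moves it at constant speed along its waypoints, reversing at either end.
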(event OnComponentHit(PaperSprite)
  (params (HitComponent :type Primitive%20Component%20Object%20Reference) (OtherActor :type Actor%20Object%20Reference) (OtherComp :type Primitive%20Component%20Object%20Reference) (NormalImpulse :type Vector :default "0, 0, 0") (Hit :type Hit%20Result%20Structure%20%28by%20ref%29))
  (bind _returnvalue (Game|GetGameMode))
  (bind _returnvalue_2 (Game|GetGameMode))
  (bind _returnvalue_3 (Game|GetGameMode))
  (bind _returnvalue_4 (Game|GetGameMode))
  (bind _asbounce_gamemode (Utilities|Casting|CastToBounceGamemode _returnvalue))
  (bind _asbounce_gamemode_2 (Utilities|Casting|CastToBounceGamemode _returnvalue_2))
  (bind _asbounce_gamemode_3 (Utilities|Casting|CastToBounceGamemode _returnvalue_3))
  (bind _asbounce_gamemode_4 (Utilities|Casting|CastToBounceGamemode _returnvalue_4))
  (bind _winscore (Variables|/Game/Blueprints/BounceGamemode.BounceGamemode_C|GetWinScore _asbounce_gamemode_3))
  (bind _widgetvar (Variables|/Game/Blueprints/BounceGamemode.BounceGamemode_C|GetWidgetVar _asbounce_gamemode_4))
  ;[1 1 1] Sets score and destroys bullet + target
  (Actor|DestroyActor OtherActor)
  (if (Variables|/Game/Blueprints/BounceGamemode.BounceGamemode_C|GetPlayer1Turn _asbounce_gamemode_2)
    (bind _output_get (Variables|/Game/Blueprints/BounceGamemode.BounceGamemode_C|SetPlayer1Score _asbounce_gamemode_2 (+ (Variables|/Game/Blueprints/BounceGamemode.BounceGamemode_C|GetPlayer1Score _asbounce_gamemode_2) 1)))
    (Rendering|Components|TextRender|SetText (Variables|/Game/Blueprints/Widgets/HUDWidget.HUDWidget_C|GetPlayer1ScoreText _widgetvar) (Utilities|Text|ToText(Integer) _output_get))
    (else
      (bind _output_get_2 (Variables|/Game/Blueprints/BounceGamemode.BounceGamemode_C|SetPlayer2Score _asbounce_gamemode_2 (+ (Variables|/Game/Blueprints/BounceGamemode.BounceGamemode_C|GetPlayer2Score _asbounce_gamemode_2) 1)))
      (Rendering|Components|TextRender|SetText (Variables|/Game/Blueprints/Widgets/HUDWidget.HUDWidget_C|GetPlayer2ScoreText _widgetvar) (Utilities|Text|ToText(Integer) _output_get_2))))
  ;[1 1 1] If player has majority of points
  (if (== _winscore (Variables|/Game/Blueprints/BounceGamemode.BounceGamemode_C|GetPlayer1Score _asbounce_gamemode_3))
    (Variables|/Game/Blueprints/BounceGamemode.BounceGamemode_C|SetPlayer1IsWinner _asbounce_gamemode_3 true)
    (Viewport|RemoveAllWidgets :!label _label)
    (bind _returnvalue_5 (UserInterface|CreateWidget "/Game/Blueprints/Widgets/GameOverScreenWidget.GameOverScreenWidget_C"))
    (bind _output_get_3 (Variables|Default|SetWinScreenVar _returnvalue_5))
    (UserInterface|Viewport|AddtoViewport _output_get_3 0)
    (if (Variables|/Game/Blueprints/BounceGamemode.BounceGamemode_C|GetPlayer1IsWinner _asbounce_gamemode)
      (Rendering|Components|TextRender|SetText (Variables|/Game/Blueprints/Widgets/GameOverScreenWidget.GameOverScreenWidget_C|GetWinnerText _output_get_3) "BLUE WINS")
      (else
        (Rendering|Components|TextRender|SetText (Variables|/Game/Blueprints/Widgets/GameOverScreenWidget.GameOverScreenWidget_C|GetWinnerText _output_get_3) "RED WINS")))
    (Rendering|Components|TextRender|SetText (Variables|/Game/Blueprints/Widgets/GameOverScreenWidget.GameOverScreenWidget_C|GetPlayer1ScoreText _output_get_3) (Utilities|Text|ToText(Integer) (Variables|/Game/Blueprints/BounceGamemode.BounceGamemode_C|GetPlayer1Score _asbounce_gamemode)))
    (Rendering|Components|TextRender|SetText (Variables|/Game/Blueprints/Widgets/GameOverScreenWidget.GameOverScreenWidget_C|GetPlayer2ScoreText _output_get_3) (Utilities|Text|ToText(Integer) (Variables|/Game/Blueprints/BounceGamemode.BounceGamemode_C|GetPlayer2Score _asbounce_gamemode)))
    (Variables|/Script/Engine.PlayerController|SetbShowMouseCursor (Game|GetPlayerController 0) true)
    (Effects|SpawnEmitteratLocation "/Game/Particles/TargetDestroyedParticles.TargetDestroyedParticles" (Transformation|GetActorLocation))
    (Audio|PlaySound2D "/Game/Audio/BulletDestroy.BulletDestroy" (Math|Conversions|ToFloat(Boolean) (Variables|/Game/Blueprints/SettingsInstance.SettingsInstance_C|GetSoundEnabled (.AsSettings%20Instance (Utilities|Casting|CastToSettingsInstance (Game|GetGameInstance))))))
    (Actor|DestroyActor)
    (Variables|/Game/Blueprints/BounceGamemode.BounceGamemode_C|SetGameIsOver (.AsBounce%20Gamemode (Utilities|Casting|CastToBounceGamemode (Game|GetGameMode))) true)
    (elif (== _winscore (Variables|/Game/Blueprints/BounceGamemode.BounceGamemode_C|GetPlayer2Score _asbounce_gamemode_3))
      (Variables|/Game/Blueprints/BounceGamemode.BounceGamemode_C|SetPlayer1IsWinner _asbounce_gamemode_3 false)
      (goto _label)
      (else
        (Effects|SpawnEmitteratLocation "/Game/Particles/TargetDestroyedParticles.TargetDestroyedParticles" (Transformation|GetActorLocation))
        (Audio|PlaySound2D "/Game/Audio/BulletDestroy.BulletDestroy" (Math|Conversions|ToFloat(Boolean) (Variables|/Game/Blueprints/SettingsInstance.SettingsInstance_C|GetSoundEnabled (.AsSettings%20Instance (Utilities|Casting|CastToSettingsInstance (Game|GetGameInstance))))))
        (Actor|DestroyActor)))))

(event EventTick
  (params (DeltaSeconds :type Float%20%28single-precision%29))
  (bind _returnvalue (Transformation|GetActorLocation))
  ;[1 1 1] Lerp target between waypoints
  (if (!= (Utilities|Array|Length (Variables|Default|GetWaypoints)) 0)
    (if (Math|Vector|Equal(Vector) _returnvalue (Transformation|GetActorLocation (Utilities|Array|Get(acopy) (Variables|Default|GetWaypoints) (Variables|Default|GetCurrentWaypoint))) 0.1)
      ;[1 1 1] Cycle waypoint
      (Variables|Default|SetCurrentWaypoint (+ (Variables|Default|GetCurrentWaypoint) (Variables|Default|GetWaypointDirection)))
      ;[1 1 1] If at end of waypoints, go the other way
      (if (or (== (Variables|Default|GetCurrentWaypoint) 0) (== (Variables|Default|GetCurrentWaypoint) (- (Utilities|Array|Length (Variables|Default|GetWaypoints)) 1)))
        (Variables|Default|SetWaypointDirection (* (Variables|Default|GetWaypointDirection) -1))))
    (Transformation|SetActorLocation (Math|Interpolation|VInterptoConstant _returnvalue (Transformation|GetActorLocation (Utilities|Array|Get(acopy) (Variables|Default|GetWaypoints) (Variables|Default|GetCurrentWaypoint))) DeltaSeconds (Variables|Default|GetSpeed)) true false)))

(fn ConstructionScript)